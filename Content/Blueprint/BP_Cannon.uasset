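; BP_Cannon is a cannon actor for a ballistics demo, with its pitch set every Tick from the degree box on BP_BallisticsFireHUD.
; Three fire events play an explosion at LaunchPos and spawn a normal projectile, a bullet or a custom bullet.
; Fire also predicts the normal projectile's path from its spawn velocity, marking it with BP_Tracker actors that are cleared after a short delay.
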(event Custom|Fire
  (bind _launchpos (Variables|Default|GetLaunchPos))
  (bind _returnvalue (Transformation|GetWorldLocation _launchpos))
  (Effects|SpawnEmitteratLocation "/Game/StarterContent/Particles/P_Explosion.P_Explosion" _returnvalue)
  (bind _returnvalue_2 (Game|SpawnActorfromClass "/Game/Blueprint/BP_NormalProjectile.BP_NormalProjectile_C" (Transformation|GetWorldTransform _launchpos) "Undefined" "MultiplyWithRoot" 0 0))
  (bind _predictresult (Class|GameplayStatics|BlueprintPredictProjectilePathAdvanced (Utilities|Struct|MakePredictProjectilePathParams _returnvalue (Transformation|GetComponentVelocity (Variables|/Script/Engine.Actor|GetRootComponent _returnvalue_2)) false 0.0 2.0 true "ECC_WorldStatic" "ObjectTypeQuery1" 0 2e+01 0.0 "None" 1.0 false)))
  (for _array_element (.pathdata _predictresult)
    (Game|SpawnActorfromClass "/Game/Blueprint/BP_Tracker.BP_Tracker_C" (Math|Transform|MakeTransform (.location _array_element) "0, 0, 0" "1.000000,1.000000,1.000000") "Undefined" "MultiplyWithRoot" 0 0)
    (Utilities|FlowControl|Delay 2.0)
    (bind _outactors (Actor|GetAllActorsOfClass "/Game/Blueprint/BP_Tracker.BP_Tracker_C"))
    (for _array_element_2 _outactors
      (Actor|DestroyActor _array_element_2))))

(event Custom|Fire2
  (bind _launchpos (Variables|Default|GetLaunchPos))
  (Effects|SpawnEmitteratLocation "/Game/StarterContent/Particles/P_Explosion.P_Explosion" (Transformation|GetWorldLocation _launchpos))
  (Game|SpawnActorfromClass "/Game/Blueprint/BP_Bullet.BP_Bullet_C" (Transformation|GetWorldTransform _launchpos) "Undefined" "MultiplyWithRoot" 0 0))

(event Custom|Fire%20Custom%20Projectile
  (bind _launchpos (Variables|Default|GetLaunchPos))
  (bind _returnvalue (Transformation|GetWorldLocation _launchpos))
  (Effects|SpawnEmitteratLocation "/Game/StarterContent/Particles/P_Explosion.P_Explosion" _returnvalue)
  (Game|SpawnActorfromClass "/Game/Blueprint/BP_CustomBullet.BP_CustomBullet_C" (Math|Transform|MakeTransform _returnvalue (Math|Rotator|MakeRotator 0.0 (.pitch (Transformation|GetActorRotation)) 0.0) "1.000000,1.000000,1.000000") "Undefined" "MultiplyWithRoot" 0 0))

(event EventBeginPlay)

(event Collision|EventActorBeginOverlap
  (params (OtherActor :type Actor%20Object%20Reference)))

(event EventTick
  (params (DeltaSeconds :type Float%20%28single-precision%29))
  (bind _returnvalue (Actor|GetActorOfClass "/Game/Blueprint/BP_BallisticsFireHUD.BP_BallisticsFireHUD_C"))
  (Transformation|SetActorRotation (Math|Rotator|MakeRotator 0.0 (Class|SpinBox|GetValue (Variables|/Game/Blueprint/BP_BallisticsFireUI.BP_BallisticsFireUI_C|GetDegBox (Variables|/Game/Blueprint/BP_BallisticsFireHUD.BP_BallisticsFireHUD_C|GetUI _returnvalue))) 0.0)))

(fn ConstructionScript)