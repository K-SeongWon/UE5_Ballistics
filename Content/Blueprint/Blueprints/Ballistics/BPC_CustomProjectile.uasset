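; Projectile component that moves its owning actor as a simulated bullet, line tracing each tick until its lifespan ends.
; A physical-material data table drives randomized penetration by speed and angle, plus energy loss through objects.
; Reverse traces find exit points for penetrations, which leave decals; other hits ricochet at half speed, and both randomly deflect.
; Gravity adjusts velocity, the drag formula is left unconnected, and optional debug lines are colored by speed.
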(event EventTick
  (params (DeltaSeconds :type Float%20%28single-precision%29))
  (if (Variables|Default|GetIsInitialized?)
    (Variables|Default|SetDeltaTime DeltaSeconds)
    (Variables|Default|SetStartPos (Transformation|GetActorLocation (Components|GetOwner)))
    (Variables|Default|SetLastPos (+ (Variables|Default|GetStartPos) (* (Variables|BulletParams|GetVelocity) (Variables|Default|GetDeltaTime))))
    (bind (_outhit _returnvalue) (Collision|LineTraceByChannel (Variables|Default|GetStartPos) (Variables|Default|GetLastPos) "TraceTypeQuery1" false (Utilities|Array|MakeArray (Variables|Default|GetActorToIgnore)) "None" true "(R=1.000000,G=0.000000,B=0.000000,A=1.000000)" "(R=0.000000,G=1.000000,B=0.000000,A=1.000000)" 1e+01))
    (if (Variables|Default|GetIsDebugLineVisible?)
      (Rendering|Debug|DrawDebugLine (Variables|Default|GetStartPos) (select _returnvalue (.ImpactPoint (Collision|BreakHitResult _outhit)) (Variables|Default|GetLastPos)) (CallFunction|GetTraceColor) 1e+01 0.0))
    (if _returnvalue
      (bind _output_get (Variables|Default|SetOut%20Hit _outhit))
      (if (CallFunction|WhethertoPenetrate (Variables|BulletParams|GetVelocity) (Variables|Default|GetOut%20Hit))
        (CallFunction|BulletHole _output_get)
        (bind (_hit _exitlocation _surfacenormal _outhit_2) (CallFunction|ComputeExitLocation (Math|Vector|Normalize (Variables|BulletParams|GetVelocity)) (Variables|Default|GetOut%20Hit)))
        (if _hit
          (if (> (CallFunction|CalculateFinalVelocity (Variables|BulletParams|GetVelocity) _exitlocation (Variables|Default|GetOut%20Hit)) 0.0)
            (Variables|Default|SetActorToIgnore (.HitActor (Collision|BreakHitResult (Variables|Default|GetOut%20Hit))))
            (CallFunction|BulletHole _outhit_2)
            (Transformation|SetActorLocation (Components|GetOwner) _exitlocation false false)
            (bind _output_get_2 (Variables|BulletParams|SetVelocity (CallFunction|ComputeGravityandDecelaration (* (Math|Vector|Normalize (Variables|BulletParams|GetVelocity)) (CallFunction|CalculateFinalVelocity (Variables|BulletParams|GetVelocity) _exitlocation (Variables|Default|GetOut%20Hit))))))
            (CallFunction|VaryTrajectory _surfacenormal _output_get_2)
            (else
              (Actor|DestroyActor (Components|GetOwner)))))
        (else
          (bind (_startpoint _velocity _impactnormal) (CallFunction|ComputeRicochet (Variables|Default|GetOut%20Hit)))
          (Variables|Default|SetActorToIgnore (.HitActor (Collision|BreakHitResult (Variables|Default|GetOut%20Hit))))
          (Transformation|SetActorLocation (Components|GetOwner) _startpoint false false)
          (bind _output_get_3 (Variables|BulletParams|SetVelocity (CallFunction|ComputeGravityandDecelaration _velocity)))
          (CallFunction|VaryTrajectory _impactnormal _output_get_3)))
      (else
        (Transformation|SetActorLocation (Components|GetOwner) (Variables|Default|GetLastPos) false false)
        (Variables|BulletParams|SetVelocity (CallFunction|ComputeGravityandDecelaration (Variables|BulletParams|GetVelocity)))))))

(event EventBeginPlay
  (Variables|BulletParams|SetVelocity (* (Transformation|GetActorForwardVector (Components|GetOwner)) (Variables|BulletParams|GetBulletSpeed)))
  (Variables|Default|SetStartPos (Transformation|GetActorLocation (Components|GetOwner)))
  (Variables|Default|SetIsInitialized? true)
  (Utilities|FlowControl|Delay (Variables|BulletParams|GetBulletLifeSpan))
  (Actor|DestroyActor (Components|GetOwner)))

(fn ComputeExitLocation
  (params (Direction :type Vector) (HitResult :type Hit%20Result%20Structure))
  (bind (_bblockinghit _binitialoverlap _time _distance _location _impactpoint _normal _impactnormal _physmat _hitactor) (Collision|BreakHitResult HitResult))
  (bind _boxextent (Collision|GetActorBounds _hitactor true true))
  (LocalVariables|SetTraceDistance (* (Math|Float|Max(Float) (.x _boxextent) (.y _boxextent) (.z _boxextent)) 4.0))
  (bind _output_get (LocalVariables|SetTraceStart (+ (* Direction (LocalVariables|GetTraceDistance)) _impactpoint)))
  (LocalVariables|SetTraceEnd (+ _output_get (* Direction (* (LocalVariables|GetTraceDistance) -1.0))))
  (bind (_outhit _returnvalue) (Collision|LineTraceByChannel (LocalVariables|GetTraceStart) (LocalVariables|GetTraceEnd) "TraceTypeQuery1" false (LocalVariables|GetIgnoreList) "None" true "(R=1.000000,G=0.996379,B=0.000000,A=1.000000)" "(R=0.000000,G=0.912769,B=1.000000,A=1.000000)" :!label _label))
  (if _returnvalue
    (if (!= (.HitActor (Collision|BreakHitResult _outhit)) _hitactor)
      (Utilities|Array|Add (LocalVariables|GetIgnoreList) (.HitActor (Collision|BreakHitResult _outhit)))
      (LocalVariables|SetTraceStart (.ImpactPoint (Collision|BreakHitResult _outhit)))
      (goto _label)
      (else
        (return true (.ImpactPoint (Collision|BreakHitResult _outhit)) (.ImpactNormal (Collision|BreakHitResult _outhit)) _outhit)))
    (else
      (return false "0, 0, 0" (.ImpactNormal (Collision|BreakHitResult _outhit)) ""))))

(fn CalculateFinalVelocity
  (params (Velocity :type Vector) (ExitLocation :type Vector) (HitResult :type Hit%20Result%20Structure))
  (bind (_bblockinghit _binitialoverlap _time _distance _location _impactpoint _normal _impactnormal _physmat) (Collision|BreakHitResult HitResult))
  (bind _returnvalue (Math|Vector|VectorLengthSquared Velocity))
  (bind _bulletmass (Variables|BulletParams|GetBulletMass))
  (bind _returnvalue_2 (* 0.5 _bulletmass _returnvalue))
  (bind _returnvalue_3 (Utilities|GetDataTableRow "/Game/Blueprint/Blueprints/Ballistics/Data.Data" (Utilities|String|StringToName (Utilities|GetObjectName _physmat)))
    (:then
      (return (Math|Float|Sqrt (/ (- _returnvalue_2 (select (> (* (Math|Vector|Distance(Vector) ExitLocation _impactpoint) _returnvalue_2 (.JoulesPerCM (Utilities|Struct|BreakPenetrationData _returnvalue_3))) _returnvalue_2) _returnvalue_2 (* (Math|Vector|Distance(Vector) ExitLocation _impactpoint) _returnvalue_2 (.JoulesPerCM (Utilities|Struct|BreakPenetrationData _returnvalue_3))))) (* 0.5 (Variables|BulletParams|GetBulletMass))))))
    (:RowNotFound
      (return (Math|Vector|VectorLength Velocity)))))

(fn WhethertoPenetrate
  (params (Velocity :type Vector) (Hit :type Hit%20Result%20Structure))
  (bind (_bblockinghit _binitialoverlap _time _distance _location _impactpoint _normal _impactnormal _physmat) (Collision|BreakHitResult Hit))
  (bind _returnvalue (Utilities|GetDataTableRow "/Game/Blueprint/Blueprints/Ballistics/Data.Data" (Utilities|String|StringToName (Utilities|GetObjectName _physmat)))
    (:then
      (return (and (> (* (Math|Float|Clamp(Float) (+ (* (Math|Vector|VectorLength Velocity) (.VelocityGradient (Utilities|Struct|BreakPenetrationData _returnvalue))) (.VelocityZIntercept (Utilities|Struct|BreakPenetrationData _returnvalue)))) (Math|Float|Clamp(Float) (+ (* (.ImpactAngleGradient (Utilities|Struct|BreakPenetrationData _returnvalue)) (CallFunction|AngleBetweenVectors (* _impactnormal -1.0) (Math|Vector|Normalize Velocity))) (.ImpactAngleZIntercept (Utilities|Struct|BreakPenetrationData _returnvalue))))) (Math|Random|RandomFloatinRange 0.0 1.0)) (> (/ (Math|Vector|VectorLength (Variables|BulletParams|GetVelocity)) (Variables|BulletParams|GetBulletSpeed)) (.MinVelocityToPenetrate (Utilities|Struct|BreakPenetrationData _returnvalue))))))
    (:RowNotFound
      (return false))))

(fn ComputeGravityandDecelaration
  (params (Velocity :type Vector))
  (return (+ Velocity (* (Math|Vector|MakeVector 0.0 0.0 (+ (Utilities|DragForce (Variables|Enviromental|GetAirDensity) (Variables|BulletParams|GetBulletSpeed) (Variables|BulletParams|GetCrossSection) (Variables|Enviromental|GetDrag%20Coefficiency)) (* (* (Variables|Enviromental|GetGravity) 1e+02) (Variables|BulletParams|GetBulletMass) -1.0))) (Variables|Default|GetDeltaTime)))))

(fn ComputeRicochet
  (params (Hit :type Hit%20Result%20Structure%20%28by%20ref%29))
  (bind (_bblockinghit _binitialoverlap _time _distance _location _impactpoint _normal _impactnormal) (Collision|BreakHitResult Hit))
  (bind _velocity (Variables|BulletParams|GetVelocity))
  (bind _returnvalue (Math|Vector|VectorLength _velocity))
  (return (+ _impactpoint _impactnormal) (Math|Vector|MirrorVectorbyNormal (* (Math|Vector|Normalize (Variables|BulletParams|GetVelocity)) (- _returnvalue (/ _returnvalue 2.0))) _impactnormal) _impactnormal))

(fn GetTraceColor
  (bind _bulletspeed (Variables|BulletParams|GetBulletSpeed))
  (bind _velocity (Variables|BulletParams|GetVelocity))
  (bind _returnvalue (Math|Vector|VectorLength _velocity))
  (bind _returnvalue_2 (/ _returnvalue _bulletspeed))
  (if (> _returnvalue_2 0.75)
    (return (Math|Color|Lerp(LinearColor) "(R=0.223228,G=0.000000,B=0.001518,A=1.000000)" "(R=0.005208,G=0.000029,B=0.000000,A=1.000000)" (* (- _returnvalue_2 0.75) 4.0)))
    (elif (> _returnvalue_2 0.5)
      (return (Math|Color|Lerp(LinearColor) "(R=1.000000,G=0.577581,B=0.000000,A=1.000000)" "(R=0.223228,G=0.000000,B=0.001518,A=1.000000)" (* (- _returnvalue_2 0.5) 4.0)))
      (elif (> _returnvalue_2 0.25)
        (return (Math|Color|Lerp(LinearColor) "(R=0.000000,G=1.000000,B=0.270498,A=1.000000)" "(R=1.000000,G=0.577581,B=0.000000,A=1.000000)" (* (- _returnvalue_2 0.25) 4.0)))
        (else
          (return (Math|Color|Lerp(LinearColor) "(R=0.708376,G=1.000000,B=0.701102,A=1.000000)" "(R=0.000000,G=1.000000,B=0.270498,A=1.000000)" (* _returnvalue_2 4.0))))))))

(fn VaryTrajectory
  (params (SurfaceNormal :type Vector) (ImpactVelocity :type Vector))
  (bind _output_get (LocalVariables|SetInitialAnswer (* (Class|KismetMathLibrary|RandomUnitVectorinConeinRadians (Variables|BulletParams|GetVelocity) (Math|Float|MapRangeClamped (Math|Vector|VectorLength ImpactVelocity) 2e+04 6e+04 0.096 0.149)) (Math|Vector|VectorLength (Variables|BulletParams|GetVelocity)))))
  (if (>= (CallFunction|AngleBetweenVectors SurfaceNormal _output_get) 9e+01)
    (Variables|BulletParams|SetVelocity (Math|Vector|RotateVector (LocalVariables|GetInitialAnswer) (* (Math|Rotator|Delta(Rotator) (Math|Rotator|MakeRotfromX SurfaceNormal) (Math|Rotator|MakeRotfromX _output_get)) (- 1.0 (/ (CallFunction|AngleBetweenVectors SurfaceNormal _output_get) 9e+01)))))
    (else
      (Variables|BulletParams|SetVelocity (LocalVariables|GetInitialAnswer))))
  (return))

(fn BulletHole
  (params (HitResult :type Hit%20Result%20Structure))
  (bind _returnvalue (Rendering|Decal|SpawnDecalatLocation (Variables|BulletHole|GetDecal%20Material) (Variables|BulletHole|GetDecal%20Size) (.location HitResult) (Math|Rotator|MakeRotfromX (.impactnormal HitResult)) (Variables|BulletHole|GetDecalLifeSpan)))
  (Rendering|Components|Decal|SetFadeScreenSize _returnvalue (Variables|BulletHole|GetDecalFadeScreenSize)))

(fn AngleBetweenVectors
  (params (V1 :type Vector) (V2 :type Vector))
  (return (Class|KismetMathLibrary|DegAcos (Math|Vector|DotProduct (Math|Vector|Normalize V1) (Math|Vector|Normalize V2)))))